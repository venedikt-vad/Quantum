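; BP_MinigameManager is an actor that cycles minigames hosted on Monitor actors in the level.
; On BeginPlay it collects all Monitors, then picks a random one that differs from the current, shows only its widget, starts it and directs the Conveyor to it.
; Success and failure both start another minigame, but success also triggers a tunnel speedup on BP_AtomPlayer.
; An unconnected FindHEX screen-widget path never runs.
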(event `InitMinigame`
  (bind _tempindex (`self.TempIndex`))
  (bind _output_get (set `self.TempIndex` (`.OutIndex` (`KismetArrayLibrary.Array_Random` (`self.MinigamesListOld`)))))
  (if (== (`|GetArrayItem` (`self.MinigamesListOld`) _output_get) (`self.CurrentMinigame`))
    (set `self.CurrentMinigame` (`|GetArrayItem` (`self.MinigamesListOld`) (mod (+ _tempindex 1) (`KismetArrayLibrary.Array_Length` (`self.MinigamesListOld`)))))
    (else
      (set `self.CurrentMinigame` (`|GetArrayItem` (`self.MinigamesListOld`) _tempindex))))
  (for _array_element (`self.MinigamesListOld`)
    (`/Game/Minigames/Monitor.SetWidgetVisible` _array_element (== _array_element (`self.CurrentMinigame`))))
  (`/Game/Minigames/Monitor.InitMinigame` (`self.CurrentMinigame`))
  (bind _returnvalue (`GameplayStatics.GetActorOfClass` "/Game/Minigames/Conveyor.Conveyor_C"))
  (`/Game/Minigames/Conveyor.MoveConveyor` _returnvalue 0 (`self.CurrentMinigame`)))

(event `MinigameSucsess`
  (`self.InitMinigame`)
  (bind _returnvalue (`GameplayStatics.GetActorOfClass` "/Game/AtomGameplay/BP_AtomPlayer.BP_AtomPlayer_C"))
  (`/Game/AtomGameplay/BP_AtomPlayer.TunnelSpeedup` _returnvalue))

(event `MinigameFail`
  (`self.InitMinigame`))

(event `self.ReceiveBeginPlay`
  (bind _outactors (`GameplayStatics.GetAllActorsOfClass` "/Game/Minigames/Monitor.Monitor_C"))
  (bind _output_get (set `self.MinigamesListOld` _outactors))
  (for _array_element _output_get
    (`KismetSystemLibrary.PrintString` (`KismetSystemLibrary.GetDisplayName` _array_element) true true (struct :`R` 1.0 :`G` 1.0 :`B` 1.0 :`A` 1.0)))
  (`self.InitMinigame`))

(fn `UserConstructionScript`)