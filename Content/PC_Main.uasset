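; Main player controller that relays arrow key input to a second player, the BP_AtomPlayer actor.
; On BeginPlay it finds and stores the first BP_AtomPlayer in the level.
; Press and release events for each of the four arrow keys call the matching press or release functions on that stored actor, so it receives input through this controller.
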(event `self.ReceiveBeginPlay`
  (bind _returnvalue (`GameplayStatics.GetActorOfClass` "/Game/AtomGameplay/BP_AtomPlayer.BP_AtomPlayer_C"))
  (set `self.AtomPlayer` _returnvalue))

(event `Key|Up`
  (params (Key :type "Key Structure"))
  (bind _atomplayer (`self.AtomPlayer`))
  ; Send Arrow Inputs to second player
  (:`Pressed`
    (`/Game/AtomGameplay/BP_AtomPlayer.UP_Press` _atomplayer))
  (:`Released`
    (`/Game/AtomGameplay/BP_AtomPlayer.UP_Release` _atomplayer)))

(event `Key|Down`
  (params (Key :type "Key Structure"))
  (bind _atomplayer (`self.AtomPlayer`))
  ; Send Arrow Inputs to second player
  (:`Pressed`
    (`/Game/AtomGameplay/BP_AtomPlayer.DOWN_Press` _atomplayer))
  (:`Released`
    (`/Game/AtomGameplay/BP_AtomPlayer.DOWN_Release` _atomplayer)))

(event `Key|Right`
  (params (Key :type "Key Structure"))
  (bind _atomplayer (`self.AtomPlayer`))
  ; Send Arrow Inputs to second player
  (:`Pressed`
    (`/Game/AtomGameplay/BP_AtomPlayer.Right_Press` _atomplayer))
  (:`Released`
    (`/Game/AtomGameplay/BP_AtomPlayer.Right_Release` _atomplayer)))

(event `Key|Left`
  (params (Key :type "Key Structure"))
  (bind _atomplayer (`self.AtomPlayer`))
  ; Send Arrow Inputs to second player
  (:`Pressed`
    (`/Game/AtomGameplay/BP_AtomPlayer.LEFT_Press` _atomplayer))
  (:`Released`
    (`/Game/AtomGameplay/BP_AtomPlayer.LEFT_Release` _atomplayer)))

(fn `UserConstructionScript`)