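; BP_GraphRender is a test graph renderer that plots a stepped sine-wave signal onto a plane through a render target.
; BeginPlay creates a canvas render target shown on the plane by an M_Graph instance and also fed into an M_GraphFrame instance.
; Each Tick passes the current and previous values plus delta time to the frame material and draws it into that same target, forming a feedback loop.
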(event `self.ReceiveBeginPlay`
  (bind _returnvalue (`CanvasRenderTarget2D.CreateCanvasRenderTarget2D` "/Script/Engine.CanvasRenderTarget2D" 256 256))
  (bind _output_get (set `self.canvas` _returnvalue))
  (bind _returnvalue_2 (`KismetMaterialLibrary.CreateDynamicMaterialInstance` "/Game/GraphRender/M_Graph.M_Graph"))
  (`MaterialInstanceDynamic.SetTextureParameterValue` _returnvalue_2 "Tex" _output_get)
  (`PrimitiveComponent.SetMaterial` (`self.Plane`) 0 _returnvalue_2)
  (bind _returnvalue_3 (`KismetMaterialLibrary.CreateDynamicMaterialInstance` "/Game/GraphRender/M_GraphFrame.M_GraphFrame"))
  (bind _output_get_2 (set `self.Mat` _returnvalue_3))
  (`MaterialInstanceDynamic.SetTextureParameterValue` _output_get_2 "Tex" _returnvalue))

(event `self.ReceiveTick`
  (params (DeltaSeconds :type "Float (single-precision)"))
  (bind _mat (`self.Mat`))
  (bind _returnvalue (/ (`/VVAD_Utils/BPF_VVAD_Utils.+1 (float)` (`KismetMathLibrary.Conv_IntToDouble` (`KismetMathLibrary.Round` (`KismetMathLibrary.Sin` (* (`GameplayStatics.GetTimeSeconds`) 10.0))))) 2.0))
  (`MaterialInstanceDynamic.SetScalarParameterValue` _mat "LastValue" (`self.LastValue`))
  (`MaterialInstanceDynamic.SetScalarParameterValue` _mat "ms" DeltaSeconds)
  (`MaterialInstanceDynamic.SetScalarParameterValue` _mat "Value" _returnvalue)
  (set `self.LastValue` _returnvalue)
  (`KismetRenderingLibrary.DrawMaterialToRenderTarget` (`self.canvas`) (`self.Mat`)))

(fn `UserConstructionScript`)