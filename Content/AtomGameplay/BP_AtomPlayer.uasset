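; Player for a tunnel level, steered by directional inputs and gamepad stick within a circular YZ cross-section using swept moves.
; Sphere overlaps slow the TunnelMover down to a minimum and flash damage on the minimap widget, with a short re-trigger cooldown.
; TunnelSpeedup, with no caller in this graph, raises tunnel speed; passing the threshold fades Project36Cue, animates camera FOV and shows the finale widget.
; The minimap is created for player controller index 1.
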(event `InputVectorAxis|Gamepad_Right2D`
  (params (AxisValue :type "Vector Structure"))
  (set `self.LastGamepadInput` AxisValue))

(event `self.ReceiveTick`
  (params (DeltaSeconds :type "Float (single-precision)"))
  (bind (_returnvalue_x _returnvalue_y _returnvalue_z) (`KismetMathLibrary.BreakVector` (`self.K2_GetActorLocation`)))
  (bind (_returnvalue_x_2 _returnvalue_y_2 _returnvalue_z_2) (`KismetMathLibrary.BreakVector` (`KismetMathLibrary.Vector_ClampSizeMax` (`KismetMathLibrary.MakeVector` 0.0 _returnvalue_y _returnvalue_z) 80.0)))
  (`self.K2_AddActorLocalOffset` (* (`KismetMathLibrary.Normal` (+ (* (`KismetMathLibrary.Vector_Up`) (`KismetMathLibrary.Conv_BoolToInt` (`self.Up`))) (* (`KismetMathLibrary.Vector_Down`) (`KismetMathLibrary.Conv_BoolToInt` (`self.Down`))) (* (`KismetMathLibrary.Vector_Left`) (`KismetMathLibrary.Conv_BoolToInt` (`self.Left`))) (* (`KismetMathLibrary.Vector_Right`) (`KismetMathLibrary.Conv_BoolToInt` (`self.Right`))) (`self.LastGamepadInput`))) 300.0 DeltaSeconds) true)
  (`self.K2_SetActorLocation` (`KismetMathLibrary.MakeVector` _returnvalue_x _returnvalue_y_2 _returnvalue_z_2)))

(event `self.Sphere.OnComponentBeginOverlap`
  (params (OverlappedComponent :type "PrimitiveComponent Object Reference") (OtherActor :type "Actor Object Reference") (OtherComp :type "PrimitiveComponent Object Reference") (OtherBodyIndex :type Integer) (bFromSweep :type Boolean) (SweepResult :type "HitResult Structure (by ref)"))
  (if true
    (`/Engine/EditorBlueprintResources/StandardMacros.DoOnce` false :!label _label
      (:`Completed`
        (`|ExecutionSequence`
          (:`then_0`
            (`self.TunnelSlowdown`)
            (`/Game/Minimap/WG_Minimap.DamageShow` (`self.WG`)))
          (:`then_1`
            (`KismetSystemLibrary.Delay` 0.5)
            (goto _label :!via `Reset`)))))))

(event `TunnelSpeedup`
  (bind _returnvalue (`GameplayStatics.GetActorOfClass` "/Script/Quantum.TunnelMover"))
  (bind _output_get (set `TunnelMover.Speed` (+ (`TunnelMover.Speed` _returnvalue) 30.0) _returnvalue))
  (if (> _output_get 550.0)
    (`AudioComponent.FadeOut` (`self.Project_36_Cue`) 5.0 0.0 "Linear")
    (bind (_direction _fov) (`Timeline|Timeline`)
      (:`Update`
        (`CameraComponent.SetFieldOfView` (`self.Camera`) _fov))
      (:`Finished`
        (bind _returnvalue_2 (`|CreateWidget` "/Game/Finale/WG_Finale.WG_Finale_C"))
        (`UserWidget.AddToViewport` _returnvalue_2 0)))))

(event `TunnelSlowdown`
  (bind _returnvalue (`GameplayStatics.GetActorOfClass` "/Script/Quantum.TunnelMover"))
  (set `TunnelMover.Speed` (`KismetMathLibrary.FMax` (+ (`TunnelMover.Speed` _returnvalue) -30.0) 50.0) _returnvalue))

(event `self.ReceiveBeginPlay`
  (bind _returnvalue (`|CreateWidget` "/Game/Minimap/WG_Minimap.WG_Minimap_C" (`GameplayStatics.GetPlayerController` 1)))
  (`UserWidget.AddToPlayerScreen` _returnvalue 0)
  (set `self.WG` _returnvalue))

(event `UP_Press`
  (set `self.Up` true))

(event `UP_Release`
  (set `self.Up` false))

(event `DOWN_Press`
  (set `self.Down` true))

(event `DOWN_Release`
  (set `self.Down` false))

(event `LEFT_Press`
  (set `self.Left` true))

(event `LEFT_Release`
  (set `self.Left` false))

(event `Right_Press`
  (set `self.Right` true))

(event `Right_Release`
  (set `self.Right` false))

(fn `UserConstructionScript`)